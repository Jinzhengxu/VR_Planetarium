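; PlanetWidget is an actor Blueprint that wraps a widget component displaying a CardPanel UI.
; It hides the panel at BeginPlay by setting its render opacity to zero.
; Two custom events, SetOpacity and SetActiveIndex, cast the component's widget to CardPanel to set its opacity or switch the page shown by its WidgetSwitcher.
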(event `self.ReceiveBeginPlay`
  (`self.SetOpacity` 0.0))

(event `SetOpacity`
  (params (Alpha :type "Float (double-precision)"))
  (bind _ascard_panel (cast `/Game/Planet/Widgets/CardPanel` (`WidgetComponent.GetWidget` (`self.Widget`))))
  (`Widget.SetRenderOpacity` _ascard_panel Alpha))

(event `SetActiveIndex`
  (params (Index :type Integer))
  (bind _ascard_panel (cast `/Game/Planet/Widgets/CardPanel` (`WidgetComponent.GetWidget` (`self.Widget`))))
  (`WidgetSwitcher.SetActiveWidgetIndex` (`/Game/Planet/Widgets/CardPanel.WidgetSwitcher` _ascard_panel) Index))

(fn `UserConstructionScript`)