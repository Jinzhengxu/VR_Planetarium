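; PlanetGroup is an actor that acts as a rotating planet selector, with child components as planets and a widget for the active one.
; Space or the Toggle Left action steps a wrapping index and yaws the group by timeline.
; Left Shift or Toggle Right zooms the selected planet in or out while fading widget opacity.
; State flags block overlapping animations, and the branch setting forward direction is unconnected.
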(event `self.ReceiveBeginPlay`
  (`self.EnableInput` (`GameplayStatics.GetPlayerController` 0))
  (set `self.Planets` (`SceneComponent.GetChildrenComponents` (`self.DefaultSceneRoot`) false)))

(event `Key|SpaceBar`
  (params (Key :type "Key Structure"))
  (bind (_returnvalue_roll _returnvalue_pitch _returnvalue_yaw) (`KismetMathLibrary.BreakRotator` (`self.K2_GetActorRotation`)))
  (bind _widget (`self.Widget`))
  (:`Pressed`
    (if (`self.IsRotating`) :!label _label
      _
      (elif (`self.IsFocusing`)
        _
        (elif (not (`self.IsScaling`))
          (set `self.IsRotating` true)
          (set `self.Index` (+ (`self.Index`) (`self.Direction`)))
          (if (> (`self.Index`) 7)
            (set `self.Index` 0))
          (if (< (`self.Index`) 0)
            (set `self.Index` 7))
          (`/Game/Planet/Blueprints/PlanetWidget.SetActiveIndex` _widget (`self.Index`))
          (`/Game/Planet/Blueprints/PlanetWidget.SetOpacity` _widget 0.0)
          (set `self.CurrentAngle` _returnvalue_yaw)
          (bind (_direction _alpha) (`Timeline|PlanetsRotationTimeLine` :!via `PlayFromStart`)
            (:`Update`
              (if (!= _alpha 0.0)
                (`self.K2_SetActorRotation` (`KismetMathLibrary.MakeRotator` 0.0 0.0 (`KismetMathLibrary.Lerp` (`self.CurrentAngle`) (+ (* (`self.RotationAngle`) (`self.Direction`)) (`self.CurrentAngle`)) _alpha)))))
            (:`Finished`
              (set `self.IsRotating` false))))))))

(event `EnhancedInput|/Game/VRTemplate/Input/Actions/IA_Menu_Toggle_Left`
  (params (ActionValue :type Boolean) (ElapsedSeconds :type "Float (double-precision)") (TriggeredSeconds :type "Float (double-precision)") (InputAction :type "InputAction Object Reference" :default "/Game/VRTemplate/Input/Actions/IA_Menu_Toggle_Left.IA_Menu_Toggle_Left"))
  (:`Started`
    (set `self.Direction` -1)
    (goto _label)))

(event `Key|LeftShift`
  (params (Key :type "Key Structure"))
  (:`Pressed`
    (if (`self.IsRotating`) :!label _label_2
      _
      (elif (`self.IsScaling`)
        _
        (elif (`self.IsFocusing`)
          (set `self.IsScaling` true)
          (bind (_direction _shrink) (`Timeline|ZoomOut` :!via `PlayFromStart`)
            (:`Update`
              (`/Game/Planet/Blueprints/PlanetWidget.SetOpacity` (`self.Widget`) _shrink)
              (`SceneComponent.SetRelativeScale3D` (`|GetArrayItem` (`self.Planets`) (`self.Index`)) (`KismetMathLibrary.Conv_DoubleToVector` (+ _shrink 1.0))))
            (:`Finished`
              (set `self.IsScaling` false)
              (set `self.IsFocusing` false)))
          (else
            (set `self.IsScaling` true)
            (set `self.IsFocusing` true)
            (bind (_direction_2 _enlarge) (`Timeline|Zoomin` :!via `PlayFromStart`)
              (:`Update`
                (`/Game/Planet/Blueprints/PlanetWidget.SetOpacity` (`self.Widget`) _enlarge)
                (`SceneComponent.SetRelativeScale3D` (`|GetArrayItem` (`self.Planets`) (`self.Index`)) (`KismetMathLibrary.Conv_DoubleToVector` (+ _enlarge 1.0))))
              (:`Finished`
                (set `self.IsScaling` false)))))))))

(event `EnhancedInput|/Game/VRTemplate/Input/Actions/IA_Menu_Toggle_Right`
  (params (ActionValue :type Boolean) (ElapsedSeconds :type "Float (double-precision)") (TriggeredSeconds :type "Float (double-precision)") (InputAction :type "InputAction Object Reference" :default "/Game/VRTemplate/Input/Actions/IA_Menu_Toggle_Right.IA_Menu_Toggle_Right"))
  (:`Started`
    (goto _label_2)))

(fn `UserConstructionScript`)